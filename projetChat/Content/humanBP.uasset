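; Human character that periodically appears in the level and catches the player's cat if it is standing.
; While the level runs, Tick counts toward a random entry time, playing a footstep sound shortly before the hidden mesh becomes visible.
; A standing cat triggers a one-time scream, then a delayed GameManager call chosen by current level.
; Otherwise the timer resets and the human hides again after a stay delay.
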(event EventTick
  (params (DeltaSeconds :type Float%20%28single-precision%29))
  (bind _gamemanager (Variables|Default|GetgameManager))
  (bind _mesh (Variables|Character|GetMesh))
  (if (Variables|Default|GetlevelStarted)
    (if (< (- (Variables|Default|GetnextEnter) (Variables|Default|GetcurrentEnter)) 3.0)
      (if (Variables|Default|GetisPlaying)
        _
        (else
          (bind _returnvalue (Audio|CreateSound2D "/Game/Cutscene/Pas_Homme.Pas_Homme" 1.0 1.0 0.0 0))
          (Audio|Components|Audio|Play _returnvalue 0.0)
          (Variables|Default|SetisPlaying true))))
    (if (== (Variables|Default|GetcurrentEnter) 0.0)
      (Variables|Default|SetnextEnter (Math|Random|RandomFloatinRange (Variables|Default|GetminValue) (Variables|Default|GetmaxValue)))
      (Variables|Default|SetcurrentEnter (+ DeltaSeconds (Variables|Default|GetcurrentEnter)))
      (else
        (Variables|Default|SetcurrentEnter (+ DeltaSeconds (Variables|Default|GetcurrentEnter)))))
    (if (> (+ DeltaSeconds (Variables|Default|GetcurrentEnter)) (Variables|Default|GetnextEnter))
      (Rendering|SetVisibility _mesh true false)
      (bind _asthird_person_cat_bp (Utilities|Casting|CastToThirdPersonCatBP (Pawn|GetControlledPawn (Game|GetPlayerController 0))))
      (if (Variables|/Game/CatBP/Blueprints/ThirdPersonCatBP.ThirdPersonCatBP_C|GetisStanding _asthird_person_cat_bp)
        (Utilities|FlowControl|DoOnce false
          (:Completed
            (bind _returnvalue_2 (Audio|CreateSound2D "/Game/Cutscene/Cri_homme.Cri_homme" 1.0 1.0 0.0 0))
            (Audio|Components|Audio|Play _returnvalue_2 0.0)
            (Utilities|FlowControl|Delay 2.0)
            (switch int (Variables|/Game/GameManager.GameManager_C|GetcurrentLevel _gamemanager)
              (:1
                (Default|Intro _gamemanager))
              (:2
                (Default|EndLevel1 _gamemanager))
              (:3
                (Default|EndLevel3 _gamemanager)))))
        (else
          (Variables|Default|SetnextEnter (Math|Random|RandomFloatinRange (Variables|Default|GetminValue) (Variables|Default|GetmaxValue)))
          (Variables|Default|SetcurrentEnter 0.0)
          (Development|PrintString "human enter")
          (Utilities|FlowControl|Delay (Variables|Default|GettimeStaying))
          (Rendering|SetVisibility _mesh false false)
          (Variables|Default|SetisPlaying false))))))

(event EventBeginPlay
  (Rendering|SetVisibility (Variables|Character|GetMesh) false false))

(fn ConstructionScript)