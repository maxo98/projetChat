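; Interior door Blueprint for modular houses that swings open while a humanBP is inside its trigger and closes when one leaves.
; Trigger overlap events play and reverse a Timeline, whose float track drives the Door component's relative yaw.
; The construction script applies the Element0 material variable to the door's first material slot.
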(event OnComponentEndOverlap(Trigger)
  (params (OverlappedComponent :type Primitive%20Component%20Object%20Reference) (OtherActor :type Actor%20Object%20Reference) (OtherComp :type Primitive%20Component%20Object%20Reference) (OtherBodyIndex :type Integer))
  (Utilities|Casting|CastTohumanBP OtherActor)
  (bind _newtrack_1 (Timeline|Timeline_0 Reverse)
    (:Update
      (Transformation|SetRelativeRotation (Variables|Default|GetDoor) (Math|Rotator|MakeRotator 0.0 0.0 _newtrack_1) false false)
      (if (>= _newtrack_1 9e+01)
        _))))

(event OnComponentBeginOverlap(Trigger)
  (params (OverlappedComponent :type Primitive%20Component%20Object%20Reference) (OtherActor :type Actor%20Object%20Reference) (OtherComp :type Primitive%20Component%20Object%20Reference) (OtherBodyIndex :type Integer) (bFromSweep :type Boolean) (SweepResult :type Hit%20Result%20Structure%20%28by%20ref%29))
  (Utilities|Casting|CastTohumanBP OtherActor)
  (bind _newtrack_1 (Timeline|Timeline_0 Play)
    (:Update
      (Transformation|SetRelativeRotation (Variables|Default|GetDoor) (Math|Rotator|MakeRotator 0.0 0.0 _newtrack_1) false false)
      (if (>= _newtrack_1 9e+01)
        _))))

(fn ConstructionScript
  (Rendering|Material|SetMaterial (Variables|Default|GetDoor) 0 (Variables|Default|GetElement%200)))