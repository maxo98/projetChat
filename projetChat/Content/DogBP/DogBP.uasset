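; Dog pawn Blueprint that walks to requested goals through AI MoveTo once it has been woken.
; The first Interact wakes it permanently through a DoOnce.
; DogTarget moves it immediately when awake, otherwise it stores the goal, which the dog heads to upon waking.
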(event Custom|Move
  (params (location :type Vector))
  (if (Variables|Default|GetisAwake)
    (AI|AIMoveTo self location 0 1e+01 true)))

(event EventInteract
  (params (player :type Third%20Person%20Cat%20BP%20Object%20Reference))
  (Utilities|FlowControl|DoOnce false
    (:Completed
      (Variables|Default|SetisAwake true)
      (if (Variables|Default|GethasToMove)
        (CallFunction|Move (Variables|Default|Gettarget))))))

(fn ConstructionScript)

(fn DogTarget
  (params (goal :type Vector))
  (if (Variables|Default|GetisAwake)
    (CallFunction|Move goal)
    (else
      (Variables|Default|SethasToMove true)
      (Variables|Default|Settarget goal))))