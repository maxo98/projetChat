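; GamelleBP is an interactable gamelle object that a player can poison and pick up.
; Interact only acts when the player has poison, with a FlipFlop alternating between two actions.
; The first sets the gamelle's HasPoison flag through a DoOnce; the second attaches it to the player and registers it as their held Gamelle.
; Debug strings report each outcome, including the lack of poison.
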(event EventInteract
  (params (player :type Third%20Person%20Cat%20BP%20Object%20Reference))
  (if (Variables|/Game/CatBP/Blueprints/ThirdPersonCatBP.ThirdPersonCatBP_C|GethasPoison player)
    (Utilities|FlowControl|FlipFlop
      (:A
        (Utilities|FlowControl|DoOnce false
          (:Completed
            (Variables|Default|SethasPoison true)
            (Development|PrintString "poison added"))))
      (:B
        (Transformation|AttachActorToActor self player "None" "KeepWorld" "KeepWorld" "KeepWorld" false)
        (Variables|/Game/CatBP/Blueprints/ThirdPersonCatBP.ThirdPersonCatBP_C|Setgamelle player self)
        (Variables|/Game/CatBP/Blueprints/ThirdPersonCatBP.ThirdPersonCatBP_C|SethasGamelle player true)
        (Development|PrintString "gamelle picked up")))
    (else
      (Development|PrintString "no poison"))))

(fn ConstructionScript)